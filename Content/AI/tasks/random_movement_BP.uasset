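; Behavior tree task that picks a random wander destination for an AI-controlled sheep.
; After a random delay of a few seconds, it turns off sprinting on the controlled sheep pawn.
; It then writes a random reachable point within a large radius of the controller's location to the destination Blackboard key and finishes successfully.
; If either cast fails, the task never calls FinishExecute.
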(event EventReceiveExecute
  (params (OwnerActor :type Actor%20Object%20Reference))
  (Utilities|FlowControl|Delay (Math|Random|RandomFloatinRange 2.0 5.0))
  (bind _assheep_controller_bp (Utilities|Casting|CastTosheep_Controller_BP OwnerActor))
  (bind _askombles_sheep_bp (Utilities|Casting|CastTokomblesSheep_BP (Pawn|GetControlledPawn _assheep_controller_bp)))
  (Variables|/Game/AI/komblesSheep_BP.komblesSheep_BP_C|SetisSprinting _askombles_sheep_bp false)
  (AI|BehaviorTree|SetBlackboardValueasVector (Variables|Default|Getdst_location) (AI|Navigation|GetRandomReachablePointinRadius (Transformation|GetActorLocation OwnerActor) 3e+04))
  (AI|BehaviorTree|FinishExecute true))