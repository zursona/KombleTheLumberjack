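; Sheep AI character that reacts to perceived Characters and switches between walking and sprinting speeds.
; Perception updates write whether a sensed Character is visible to the kombleVisible blackboard key.
; Tick sets max walk speed from IsSprinting, which is not set in this graph.
; When not sprinting, it plays a sheep sound at the world origin, latched by IsSheepShouting, which is never reset here.
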(event OnTargetPerceptionUpdated(AIPerception)
  (params (Actor :type Actor%20Object%20Reference) (Stimulus :type AI%20Stimulus%20Structure))
  (Utilities|Casting|CastToCharacter Actor)
  (AI|Components|Blackboard|SetValueasBool (AI|GetBlackboard 0) (Utilities|Name|MakeLiteralName "kombleVisible") (.bSuccessfullySensed (Utilities|Struct|BreakAIStimulus Stimulus))))

(event EventBeginPlay)

(event EventTick
  (params (DeltaSeconds :type Float%20%28single-precision%29))
  (bind _charactermovement (Variables|Character|GetCharacterMovement))
  (if (Variables|Default|GetisSprinting)
    (Variables|/Script/Engine.CharacterMovementComponent|SetMaxWalkSpeed _charactermovement 3e+03)
    (else
      (Variables|/Script/Engine.CharacterMovementComponent|SetMaxWalkSpeed _charactermovement 6e+02)
      (if (not (Variables|Default|GetisSheepShouting))
        (Audio|PlaySoundatLocation "/Game/Sound/AI_sheepSounds.AI_sheepSounds" "0, 0, 0")
        (Variables|Default|SetisSheepShouting true)))))

(fn ConstructionScript)