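; A flower spawn area actor that scatters child actors, by its naming flowers, at random points inside a box.
; The Construction Script sizes the FlowerArea box from FlowerSpawnBoxArea, then calls SpawnFlowers, which loops up to FlowerMaxCount adding Child Actor Components at random positions within the box extent.
; Placement happens at construction, so the layout re-randomizes whenever the script reruns; the event graph holds no active logic.
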(event EventBeginPlay)

(event Collision|EventActorBeginOverlap
  (params (OtherActor :type Actor%20Object%20Reference)))

(event EventTick
  (params (DeltaSeconds :type Float%20%28single-precision%29)))

(fn ConstructionScript
  (Components|Box|SetBoxExtent (Variables|Default|GetflowerArea) (Variables|Default|GetflowerSpawnBoxArea) true)
  (CallFunction|SpawnFlowers))

(fn SpawnFlowers
  (bind _flowerarea (Variables|Default|GetflowerArea))
  (for _index (range 0 (Variables|Default|GetflowerMaxCount))
    (AddComponent|AddChildActorComponent false (Math|Conversions|ToTransform(Vector) (Math|Random|RandomPointinBoundingBox (Variables|/Script/Engine.SceneComponent|GetRelativeLocation _flowerarea) (Components|Box|GetScaledBoxExtent _flowerarea))))))